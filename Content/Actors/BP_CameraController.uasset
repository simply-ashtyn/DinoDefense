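; Camera controller actor that pans across the world's horizontal plane by touch dragging.
; BeginPlay shows the mouse cursor, and pressing the MoveCamera action records the Touch1 screen position as the drag start.
; Every Tick, without checking whether the touch is held, it converts the screen delta since the last position into an unswept world offset, swapping axes and negating vertical movement, then stores the new position.
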(event EventBeginPlay
  (Variables|/Script/Engine.PlayerController|SetbShowMouseCursor (Game|GetPlayerController 0) true))

(event EventTick
  (params (DeltaSeconds :type Float%20%28single-precision%29))
  (bind _returnvalue (Game|GetPlayerController 0))
  (bind (_locationx _locationy) (Class|PlayerController|GetInputTouchState _returnvalue "Touch1"))
  (if true
    (bind _output_get (Variables|Default|SetNewClickLocation (Math|Vector2D|MakeVector2D _locationx _locationy)))
    (Transformation|AddActorWorldOffset (Math|Vector|MakeVector (* (.y (- (Variables|Default|GetNewClickLocation) (Variables|Default|GetPreviousClickLocation))) -1.0) (* (.x (- (Variables|Default|GetNewClickLocation) (Variables|Default|GetPreviousClickLocation))) 1.0) 0.0))
    (Variables|Default|SetPreviousClickLocation _output_get)))

(event Input|ActionEvents|InputActionMoveCamera
  (params (Key :type Key%20Structure :default "None"))
  (bind _returnvalue (Game|GetPlayerController 0))
  (bind (_locationx _locationy) (Class|PlayerController|GetInputTouchState _returnvalue "Touch1"))
  (:Pressed
    (Variables|Default|SetPreviousClickLocation (Math|Vector2D|MakeVector2D _locationx _locationy))))

(event Input|ActionEvents|InputActionRotateCamera
  (params (Key :type Key%20Structure :default "None")))

(fn ConstructionScript)